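; Master building actor for the building system, starting as a ghost preview with a build widget and resource-specific versions.
; ChangeResource retints the dynamic ghost material and refreshes the widget from the ResourceVersion map.
; OnBuild enables blocking collision, applies the resource's material and swaps the widget for a health bar.
; A looping timer then raises health through BPCBuildingStats until construction ends at full health or after the build time.
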(event Custom|SetCanBeBuilt
  (params (New%20Value :type Boolean))
  (bind _output_get (Variables|Default|SetCanBeBuilt? New%20Value))
  (Default|SetCanbeBuilt (Variables|Default|GetBuildWidgetReference) _output_get))

(event Custom|OnBuild
  (params (Resource :type BP%20Master%20Resource%20Class%20Reference))
  (bind _bpc_buildingstats (Variables|Default|GetBPC_BuildingStats))
  (bind _resourceversion (Variables|Default|GetResourceVersion))
  (bind _interval (Variables|Default|GetInterval))
  (bind _buildingmesh (Variables|Default|GetBuildingMesh))
  (bind _value (Utilities|Map|Find _resourceversion Resource))
  (bind (_requiredamount _buildingtime _maximumhealth) (Utilities|Struct|BreakS_BuildingResourceVersion _value))
  (if (Utilities|IsValidClass Resource)
    (Variables|Default|SetBuilt? true)
    (Collision|SetCollisionResponsetoAllChannels _buildingmesh "ECR_Block")
    (Rendering|Material|SetMaterial _buildingmesh 0 (Utilities|Struct|BreakS_ResourceData (Utilities|GetClassDefaults Resource)))
    (Components|DestroyComponent (Variables|Default|GetBuildWidget))
    (Default|SetMaxStatValue _bpc_buildingstats "NewEnumerator0" _maximumhealth false)
    (Default|SetStat _bpc_buildingstats "NewEnumerator0" 0 false)
    (Variables|Default|SetBuildingTime _buildingtime)
    (Default|InitializeBar (Variables|Default|GetHealthBarRef) (Default|GetMaxHealth _bpc_buildingstats))
    (Rendering|SetVisibility (Variables|Default|GetHealthBar) true false)
    (bind _returnvalue (Utilities|Time|SetTimerbyEvent (delegate Custom|BuildingTick) _interval true))
    (Variables|Default|SetBuildingTimerHandle _returnvalue)
    (Utilities|FlowControl|Delay (+ (Variables|Default|GetBuildingTime) _interval))
    (CallFunction|OnBuildingEnd)))

(event Custom|BuildingTick
  (bind _bpc_buildingstats (Variables|Default|GetBPC_BuildingStats))
  (bind _out (Default|GetMaxHealth _bpc_buildingstats))
  (Default|ModifyStat _bpc_buildingstats "NewEnumerator2" (Math|Float|Ceil (/ (Math|Conversions|ToFloat(Integer) _out) (Math|Conversions|ToFloat(Integer) (Math|Float|Floor (/ (Variables|Default|GetBuildingTime) (Variables|Default|GetInterval)))))))
  (if (== (.CurrentValue (Default|GetStat _bpc_buildingstats "NewEnumerator2")) _out)
    (CallFunction|OnBuildingEnd)))

(event Custom|OnBuildingEnd
  (bind _buildingtimerhandle (Variables|Default|GetBuildingTimerHandle))
  (if (Utilities|Time|IsValidTimerHandle _buildingtimerhandle)
    (Utilities|Time|ClearandInvalidateTimerbyHandle _buildingtimerhandle)
    (Default|SetState (Variables|Default|GetHealthBarRef) "NewEnumerator1")))

(event EventBeginPlay
  (bind _buildingmesh (Variables|Default|GetBuildingMesh))
  (bind _resource (Variables|Default|GetResource))
  (bind _returnvalue (Rendering|Material|CreateDynamicMaterialInstance _buildingmesh 0 (Rendering|Material|GetMaterial _buildingmesh 0) "None" :!class /Script/Engine.PrimitiveComponent))
  (Variables|Default|SetDynamicMaterial _returnvalue)
  (CallFunction|UpdateGhostMaterial)
  (bind _asw_build_widget (Utilities|Casting|CastToW_BuildWidget (UserInterface|GetUserWidgetObject (Variables|Default|GetBuildWidget))))
  (bind _output_get (Variables|Default|SetBuildWidgetReference _asw_build_widget))
  (bind _asw_building_health_bar (Utilities|Casting|CastToW_BuildingHealthBar (UserInterface|GetUserWidgetObject (Variables|Default|GetHealthBar))))
  (Variables|Default|SetHealthBarRef _asw_building_health_bar)
  (Default|Update _output_get (.Value (Utilities|Map|Find (Variables|Default|GetResourceVersion) _resource)) _resource)
  (Default|InitializeManager (Variables|Default|GetBPC_BuildingStats) self)
  (Rendering|SetVisibility (Variables|Default|GetBuildWidget) true false))

(event Collision|EventActorBeginOverlap
  (params (OtherActor :type Actor%20Object%20Reference)))

(event EventTick
  (params (DeltaSeconds :type Float%20%28single-precision%29)))

(fn ConstructionScript)

(fn UpdateGhostMaterial
  (Rendering|Material|SetVectorParameterValue (Variables|Default|GetDynamicMaterial) "Color" (Utilities|Struct|BreakS_ResourceData (Utilities|GetClassDefaults (Variables|Default|GetResource))) :!class /Script/Engine.MaterialInstanceDynamic)
  (return))

(fn ChangeResource
  (params (New%20Resource :type BP%20Master%20Resource%20Class%20Reference))
  (if (and (Utilities|IsValidClass New%20Resource) (!= (Variables|Default|GetResource) New%20Resource))
    (Variables|Default|SetResource New%20Resource)
    (CallFunction|UpdateGhostMaterial)
    (Default|Update (Variables|Default|GetBuildWidgetReference) (.Value (Utilities|Map|Find (Variables|Default|GetResourceVersion) (Variables|Default|GetResource))) (Variables|Default|GetResource))
    (return)
    (else
      (return))))