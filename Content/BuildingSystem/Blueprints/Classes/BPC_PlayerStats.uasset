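; Player stats component that links stat values to the Health and Shield bars on the player's main widget.
; InitializeManager stores the player reference and calls SetUpStats, whose logic is not defined in this graph.
; OnStatsSetUp initializes a bar for each key in the Stats map, and UpdateStats pushes a changed stat's current value to its bar.
; GetBarForStat selects the widget bar matching each stat.
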(event Custom|InitializeManager
  (params (Player :type Third%20Person%20Character%20Object%20Reference))
  (Variables|Default|SetPlayerRef Player)
  (CallFunction|SetUpStats))

(event EventBeginPlay
  (|CallParentFunction) ; This node is disabled and will not be called.\nDrag off pins to build functionality.
)

(event EventTick
  (params (DeltaSeconds :type Float%20%28single-precision%29))
  (|CallParentFunction DeltaSeconds) ; This node is disabled and will not be called.\nDrag off pins to build functionality.
)

(event EventOnStatsSetUp
  (bind _keys (Utilities|Map|Keys (Variables|Default|GetStats)))
  (for _array_element _keys
    (Default|InitializeBar (CallFunction|GetBarforStat _array_element) (.StatValue (CallFunction|GetStat _array_element)))))

(event EventUpdateStats
  (params (Stat :type E_Stats%20Enum :default "NewEnumerator0"))
  (Default|UpdateStat (CallFunction|GetBarforStat Stat) (.CurrentValue (CallFunction|GetStat Stat))))

(fn GetBarforStat
  (params (Stat :type E_Stats%20Enum :default "NewEnumerator0"))
  (bind _playerref (Variables|Default|GetPlayerRef))
  (bind _mainwidget (Variables|/Game/ThirdPersonBP/Blueprints/ThirdPersonCharacter.ThirdPersonCharacter_C|GetMainWidget _playerref))
  (return (Utilities|Select :Index Stat :NewEnumerator0 0 :NewEnumerator1 (Variables|/Game/BuildingSystem/Widgets/W_Main.W_Main_C|GetShieldBar _mainwidget) :NewEnumerator2 (Variables|/Game/BuildingSystem/Widgets/W_Main.W_Main_C|GetHealthBar _mainwidget))))