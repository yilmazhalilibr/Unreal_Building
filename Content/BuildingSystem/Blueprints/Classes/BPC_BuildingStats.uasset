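; Building component that manages stats for a building in the building system, stored as a map of min, current and max values.
; InitializeManager caches the owning building and calls SetUpStats.
; SetMaxStatValue rewrites a stat's entry with its current value clamped, optionally calling UpdateStats.
; UpdateStats refreshes the health bar when the health stat changes and the building is in player sight.
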(event Custom|InitializeManager
  (params (Building :type BP%20Master%20Building%20Object%20Reference))
  (Utilities|IsValid Building
    (:Is%20Valid
      (Variables|Default|SetBuilding Building)
      (CallFunction|SetUpStats))))

(event EventBeginPlay
  (|CallParentFunction) ; This node is disabled and will not be called.\nDrag off pins to build functionality.
)

(event EventTick
  (params (DeltaSeconds :type Float%20%28single-precision%29))
  (|CallParentFunction DeltaSeconds) ; This node is disabled and will not be called.\nDrag off pins to build functionality.
)

(event EventUpdateStats
  (params (Stat :type E_Stats%20Enum :default "NewEnumerator0"))
  (if (and (Utilities|Enum|Equal(Enum) Stat "NewEnumerator2") (Variables|/Game/BuildingSystem/Blueprints/Classes/BP_Master_Building.BP_Master_Building_C|GetInPlayerSight? (Variables|Default|GetBuilding)))
    (Default|UpdateHealth (Variables|/Game/BuildingSystem/Blueprints/Classes/BP_Master_Building.BP_Master_Building_C|GetHealthBarRef (Variables|Default|GetBuilding)) (.CurrentValue (CallFunction|GetStat "NewEnumerator2")))))

(fn GetMaxHealth
  (return (Utilities|Struct|BreakS_StatValue (.StatValue (CallFunction|GetStat "NewEnumerator2")))))

(fn SetMaxStatValue
  (params (Stat :type E_Stats%20Enum :default "NewEnumerator0") (New%20value :type Integer) (Update? :type Boolean))
  (LocalVariables|SetlocalStat Stat)
  (LocalVariables|SetlocalUpdate false)
  (LocalVariables|SetlocalValue 0)
  (bind _keys (Utilities|Map|Keys (Variables|Default|GetStats)))
  (if (and (Utilities|Array|ContainsItem _keys (LocalVariables|GetlocalStat)) (Utilities|Enum|NotEqual(Enum) (LocalVariables|GetlocalStat) "NewEnumerator0"))
    (Utilities|Map|Add (Variables|Default|GetStats) (LocalVariables|GetlocalStat) (Utilities|Struct|MakeS_StatValue (.MinValue (Utilities|Struct|BreakS_StatValue (.StatValue (CallFunction|GetStat (LocalVariables|GetlocalStat))))) (Math|Integer|Clamp(Integer) (.CurrentValue (CallFunction|GetStat (LocalVariables|GetlocalStat))) (.MinValue (Utilities|Struct|BreakS_StatValue (.StatValue (CallFunction|GetStat (LocalVariables|GetlocalStat))))) (LocalVariables|GetlocalValue)) (LocalVariables|GetlocalValue)))
    (if (LocalVariables|GetlocalUpdate)
      (CallFunction|UpdateStats (LocalVariables|GetlocalStat))
      (return)
      (else
        (return)))
    (else
      (return))))