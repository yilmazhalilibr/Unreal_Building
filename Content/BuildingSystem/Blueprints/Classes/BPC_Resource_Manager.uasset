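; Actor component for the building system that stores resource amounts in a map keyed by resource class.
; AddResource and RemoveResource validate the class and a positive amount, then write back a clamped total, so removal never empties or deletes an entry.
; GetResource returns the stored amount, or -1 for an unknown resource.
; Successful changes call UpdateResourceDisplay, which is an empty stub here.
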(event EventBeginPlay)

(event EventTick
  (params (DeltaSeconds :type Float%20%28single-precision%29)))

(fn GetResource
  (params (Resource :type BP%20Master%20Resource%20Class%20Reference))
  (bind _resources (Variables|Default|GetResources))
  (bind (_value _returnvalue) (Utilities|Map|Find _resources Resource))
  (if _returnvalue
    (return _value)
    (else
      (return -1))))

(fn UpdateResourceDisplay
  (params (Resource :type BP%20Master%20Resource%20Class%20Reference)))

(fn AddResource
  (params (Resource :type BP%20Master%20Resource%20Class%20Reference) (Amount :type Integer))
  (bind _resources (Variables|Default|GetResources))
  (LocalVariables|SetlocalResource Resource)
  (LocalVariables|SetlocalAmount Amount)
  (if (and (Utilities|IsValidClass Resource) (> Amount 0))
    (if (.ReturnValue (Utilities|Map|Find (Variables|Default|GetResources) (LocalVariables|GetlocalResource)))
      (Utilities|Map|Add _resources (LocalVariables|GetlocalResource) (Math|Integer|Clamp(Integer) (+ (.Value (Utilities|Map|Find (Variables|Default|GetResources) (LocalVariables|GetlocalResource))) (LocalVariables|GetlocalAmount)) 1 100))
      (else
        (Utilities|Map|Add _resources (LocalVariables|GetlocalResource) (Math|Integer|Clamp(Integer) (LocalVariables|GetlocalAmount) 1 100))))
    (CallFunction|UpdateResourceDisplay (LocalVariables|GetlocalResource))
    (return)
    (else
      (return))))

(fn RemoveResource
  (params (Resource :type BP%20Master%20Resource%20Class%20Reference) (Amount :type Integer))
  (LocalVariables|SetlocalResource Resource)
  (LocalVariables|SetlocalAmount Amount)
  (if (and (Utilities|IsValidClass Resource) (> Amount 0))
    (if (.ReturnValue (Utilities|Map|Find (Variables|Default|GetResources) (LocalVariables|GetlocalResource)))
      (Utilities|Map|Add (Variables|Default|GetResources) (LocalVariables|GetlocalResource) (Math|Integer|Clamp(Integer) (- (.Value (Utilities|Map|Find (Variables|Default|GetResources) (LocalVariables|GetlocalResource))) (LocalVariables|GetlocalAmount)) 1 100))
      (CallFunction|UpdateResourceDisplay (LocalVariables|GetlocalResource))
      (return)
      (else
        (return)))
    (else
      (return))))